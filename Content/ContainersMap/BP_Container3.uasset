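; BP_Container3 is a container actor on the containers map that moves its Cube component around a fixed looping route.
; BeginPlay starts the MovementC3 custom event, which alternates delays with timed MoveComponentTo steps through hard-coded relative locations at a constant target rotation.
; Each step shifts the cube along Y or Z until it returns to its origin, where the event calls itself to repeat indefinitely.
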(event Custom|MovementC3
  (Utilities|FlowControl|Delay 1e+01)
  (Components|MoveComponentTo (Variables|Default|GetCube) "0,1000.000000, 0" "0,90.000000, 0" false false 6.0 false)
  (Utilities|FlowControl|Delay 1e+01)
  (Components|MoveComponentTo (Variables|Default|GetCube) "0,1000.000000,150.000000" "0,90.000000, 0" false false 6.0 false)
  (Utilities|FlowControl|Delay 1e+01)
  (Components|MoveComponentTo (Variables|Default|GetCube) "0,-500.000000,150.000000" "0,90.000000, 0" false false 6.0 false)
  (Utilities|FlowControl|Delay 1e+01)
  (Components|MoveComponentTo (Variables|Default|GetCube) "0,-500.000000,-450.000000" "0,90.000000, 0" false false 6.0 false)
  (Utilities|FlowControl|Delay 1e+01)
  (Components|MoveComponentTo (Variables|Default|GetCube) "0,0.000000,-450.000000" "0,90.000000, 0" false false 6.0 false)
  (Utilities|FlowControl|Delay 1e+01)
  (Components|MoveComponentTo (Variables|Default|GetCube) "0, 0, 0" "0,90.000000, 0" false false 6.0 false)
  (CallFunction|MovementC3))

(event EventBeginPlay
  (CallFunction|MovementC3))

(fn ConstructionScript)