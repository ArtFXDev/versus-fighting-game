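; BP_Container1 is a moving container actor for the containers map that cycles its Cube component through a fixed path.
; BeginPlay starts MovementC1, which chains delayed, timed MoveComponentTo steps through six offsets along Y and Z at a constant rotation, then calls itself to repeat.
; Each target adds an offset to the actor's current world location, yet is passed as a relative location.
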(event Custom|MovementC1
  (Utilities|FlowControl|Delay 1e+01)
  (Components|MoveComponentTo (Variables|Default|GetCube) (+ (Transformation|GetActorLocation) "0,1000.000000, 0") "0,90.000000, 0" false false 6.0 false)
  (Utilities|FlowControl|Delay 1e+01)
  (Components|MoveComponentTo (Variables|Default|GetCube) (+ (Transformation|GetActorLocation) "0,1000.000000,-250.000000") "0,90.000000, 0" false false 6.0 false)
  (Utilities|FlowControl|Delay 1e+01)
  (Components|MoveComponentTo (Variables|Default|GetCube) (+ (Transformation|GetActorLocation) "0,-300.000000,-250.000000") "0,90.000000, 0" false false 6.0 false)
  (Utilities|FlowControl|Delay 1e+01)
  (Components|MoveComponentTo (Variables|Default|GetCube) (+ (Transformation|GetActorLocation) "0,-600.000000,-250.000000") "0,90.000000, 0" false false 6.0 false)
  (Utilities|FlowControl|Delay 1e+01)
  (Components|MoveComponentTo (Variables|Default|GetCube) (+ (Transformation|GetActorLocation) "0,-100.000000,0.000000") "0,90.000000, 0" false false 6.0 false)
  (Utilities|FlowControl|Delay 1e+01)
  (Components|MoveComponentTo (Variables|Default|GetCube) (+ (Transformation|GetActorLocation) "0,-0.000000,0.000000") "0,90.000000, 0" false false 6.0 false)
  (CallFunction|MovementC1))

(event EventBeginPlay
  (CallFunction|MovementC1))

(fn ConstructionScript)