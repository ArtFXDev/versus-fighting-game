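; BP_Container2 is a moving container for the containers map that shifts its Cube component along a fixed looping route.
; On BeginPlay, MovementC2 chains latent MoveComponentTo steps, each preceded by a pause, sliding the cube through hardcoded relative Y and Z waypoints at constant rotation.
; After returning to the relative origin, the event calls itself to repeat the cycle indefinitely.
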(event Custom|MovementC2
  (Utilities|FlowControl|Delay 1e+01)
  (Components|MoveComponentTo (Variables|Default|GetCube) "0,750.000000, 0" "0,90.000000, 0" false false 6.0 false)
  (Utilities|FlowControl|Delay 1e+01)
  (Components|MoveComponentTo (Variables|Default|GetCube) "0,750.000000,-150.000000" "0,90.000000, 0" false false 6.0 false)
  (Utilities|FlowControl|Delay 1e+01)
  (Components|MoveComponentTo (Variables|Default|GetCube) "0,-400.000000,-150.000000" "0,90.000000, 0" false false 6.0 false)
  (Utilities|FlowControl|Delay 1e+01)
  (Components|MoveComponentTo (Variables|Default|GetCube) "0,-400.000000,-400.000000" "0,90.000000, 0" false false 6.0 false)
  (Utilities|FlowControl|Delay 1e+01)
  (Components|MoveComponentTo (Variables|Default|GetCube) "0,0.000000,-400.000000" "0,90.000000, 0" false false 6.0 false)
  (Utilities|FlowControl|Delay 1e+01)
  (Components|MoveComponentTo (Variables|Default|GetCube) "0,0.000000, 0" "0,90.000000, 0" false false 6.0 false)
  (CallFunction|MovementC2))

(event EventBeginPlay
  (CallFunction|MovementC2))

(fn ConstructionScript)