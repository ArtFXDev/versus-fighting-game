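; BP_Text is a showcase text actor in the Explosions Mega Pack that displays a title and two description lines.
; Its construction script copies the text variables into three text render components, then applies a shared horizontal alignment and color to all of them.
; The file shows only this construction-time setup, with no runtime logic.
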(fn ConstructionScript
  (bind _textrender_title (Variables|Default|GetTextRender_Title))
  (Utilities|FlowControl|Sequence
    (:then_0
      ;[1 1 1] Here we set the text for the title, the 1st and 2nd lines from the text variables
      (Rendering|Components|TextRender|SetText _textrender_title (Variables|Customize|GetTextTitle))
      (Rendering|Components|TextRender|SetText (Variables|Default|GetTextRender_Description_01) (Variables|Customize|GetTextDescriptionLine01))
      (Rendering|Components|TextRender|SetText (Variables|Default|GetTextRender_Description_02) (Variables|Customize|GetTextDescriptionLine02)))
    (:then_1
      ;[1 1 1] Here we set the text alignment
      (Rendering|Components|TextRender|SetHorizontalAlignment _textrender_title (Variables|Customize|GetAlignment)))
    (:then_2
      ;[1 1 1] And here we set the text color
      (Rendering|Components|TextRender|SetTextRenderColor (Variables|Default|GetTextRender_Title) (Math|Conversions|ToColor(LinearColor) (Variables|Customize|GetTextColor))))))