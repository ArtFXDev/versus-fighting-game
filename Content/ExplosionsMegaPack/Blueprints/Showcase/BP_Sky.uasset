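; Showcase sky actor that switches between time-of-day lighting presets via number keys, starting in evening on BeginPlay.
; Each preset calls ChangeDayTime, which caches the current sun rotation, sun color and skylight intensity.
; A timeline then blends the DirectionalLight and SkyLight from those values to the new ones.
; Holding Q slows global time, and P toggles game pause.
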(event Custom|ChangeDayTime
  (params (Sun%20Rotation :type Rotator) (Sun%20Color :type Linear%20Color%20Structure) (SkyLight%20Intensity :type Float%20%28single-precision%29))
  (bind _directionallight (Variables|Default|GetDirectionalLight))
  (bind _directionallight_2 (Variables|Default|GetDirectionalLight))
  ;[1 1 1] First we store the current values for the Directional and the Sky Light in order to smoothly blend between the different times of day
  (Variables|Default|SetTempSunRotation (Variables|/Script/Engine.SceneComponent|GetRelativeRotation _directionallight))
  (Variables|Default|SetTempSunColor (Rendering|Components|Light|GetLightColor _directionallight))
  (Variables|Default|SetTempSkyIntensity (Variables|/Script/Engine.LightComponentBase|GetIntensity (Variables|Default|GetSkyLight)))
  ;[1 1 1] This timeline lerps between the current and the new values
  (bind _lerp (Timeline|Timeline_ChangeDaytime PlayFromStart)
    (:Update
      ;[1 1 1] First, we change the Directional Light / Sun rotation (order not important)
      (Transformation|SetRelativeRotation _directionallight_2 (Math|Rotator|Lerp(Rotator) (Variables|Default|GetTempSunRotation) Sun%20Rotation _lerp true) false false)
      ;[1 1 1] Then we change the Directional Light color
      (Rendering|Components|Light|SetLightColor _directionallight_2 (Math|Color|Lerp(LinearColor) (Variables|Default|GetTempSunColor) Sun%20Color _lerp) true)
      ;[1 1 1] And at the end we change the Skylight intensity
      (Rendering|Components|Light|SetIntensity (Variables|Default|GetSkyLight) (Math|Float|Lerp (Variables|Default|GetTempSkyIntensity) SkyLight%20Intensity _lerp)))))

(event EventBeginPlay
  ;[1 1 1] When the game starts we change the time of day to evening
  ;[1 1 1] Cycling through different daytimes depending on what key the player presses
  (CallFunction|ChangeDayTime "-155.000000, 0, 0" "(R=0.470588,G=0.165642,B=0.051764,A=1.000000)" 1.0))

(event Input|KeyboardEvents|1
  (params (Key :type Key%20Structure :default "AnyKey"))
  ;[1 1 1] Cycling through different daytimes depending on what key the player presses
  (:Pressed
    (CallFunction|ChangeDayTime "-90.000000, 0, 0" "(R=1.000000,G=1.000000,B=1.000000,A=1.000000)" 5.0)))

(event Input|KeyboardEvents|2
  (params (Key :type Key%20Structure :default "AnyKey"))
  ;[1 1 1] Cycling through different daytimes depending on what key the player presses
  (:Pressed
    (CallFunction|ChangeDayTime "-130.000000, 0, 0" "(R=0.725490,G=0.504284,B=0.363296,A=1.000000)" 2.0)))

(event Input|KeyboardEvents|5
  (params (Key :type Key%20Structure :default "AnyKey"))
  ;[1 1 1] Cycling through different daytimes depending on what key the player presses
  (:Pressed
    (CallFunction|ChangeDayTime "-179.000000, 0, 0" "(R=0.405000,G=0.000000,B=0.003987,A=1.000000)" 0.25)))

(event Input|KeyboardEvents|6
  (params (Key :type Key%20Structure :default "AnyKey"))
  ;[1 1 1] Cycling through different daytimes depending on what key the player presses
  (:Pressed
    (CallFunction|ChangeDayTime "-180.000000, 0, 0" "(R=0.052000,G=0.057273,B=0.100000,A=1.000000)" 0.1)))

(event Input|KeyboardEvents|3
  (params (Key :type Key%20Structure :default "AnyKey"))
  ;[1 1 1] Cycling through different daytimes depending on what key the player presses
  (:Pressed
    (CallFunction|ChangeDayTime "-155.000000, 0, 0" "(R=0.470588,G=0.165642,B=0.051764,A=1.000000)" 1.0)))

(event Input|KeyboardEvents|P
  (params (Key :type Key%20Structure :default "AnyKey"))
  ;[1 1 1] Pause / Unpause the game
  (:Pressed
    (Utilities|FlowControl|FlipFlop
      (:A
        (Game|SetGamePaused true))
      (:B
        (Game|SetGamePaused false)))))

(event Input|KeyboardEvents|4
  (params (Key :type Key%20Structure :default "AnyKey"))
  ;[1 1 1] Cycling through different daytimes depending on what key the player presses
  (:Pressed
    (CallFunction|ChangeDayTime "-170.000000, 0, 0" "(R=0.603922,G=0.129412,B=0.019608,A=1.000000)" 0.5)))

(event Input|KeyboardEvents|Q
  (params (Key :type Key%20Structure :default "AnyKey"))
  ;[1 1 1] When the player holds down "Q" we slowdown the time, when he releases the key we set it back to the default value of 1
  (:Pressed
    (Utilities|Time|SetGlobalTimeDilation 0.2))
  (:Released
    (Utilities|Time|SetGlobalTimeDilation 1.0)))

(fn ConstructionScript)