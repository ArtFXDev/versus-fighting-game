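; Showcase grenade actor that explodes on its first collider overlap or 0.75 seconds after BeginPlay, whichever comes first.
; A DoOnce shared by both triggers ensures a single explosion.
; Explode runs a sphere trace around the actor: a nearby hit spawns a directional emitter aligned to the surface normal, otherwise a radial one spawns.
; The actor then destroys itself.
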(event OnComponentBeginOverlap(CollisionComponent)
  (params (OverlappedComponent :type Primitive%20Component%20Object%20Reference) (OtherActor :type Actor%20Object%20Reference) (OtherComp :type Primitive%20Component%20Object%20Reference) (OtherBodyIndex :type Integer) (bFromSweep :type Boolean) (SweepResult :type Hit%20Result%20Structure%20%28by%20ref%29))
  ;[1 1 1] If the collider overlaps with a prop we trigger the explosion
  ;[1 1 1] This makes sure that the explosion triggers only once
  (Utilities|FlowControl|DoOnce false
    (:Completed
      (CallFunction|Explode))))

(event Custom|Explode
  (bind _returnvalue (Transformation|GetActorLocation))
  (bind _returnvalue_2 (Transformation|GetActorLocation))
  ;[1 1 1] We use a sphere trace around the explosion to check for props
  (bind _outhit (Collision|SphereTraceForObjects _returnvalue_2 _returnvalue_2 1e+02 (Variables|Default|GetObjectType) false 0 "None"))
  (if (.bblockinghit _outhit)
    ;[1 1 1] If there's an object nearby we spawn the directional version
    (Effects|SpawnEmitteratLocation (Variables|Default|GetEmitterToSpawnDirectional) _returnvalue (Math|Rotator|MakeRotfromZ (.normal _outhit)))
    (else
      ;[1 1 1] If not, we spawn the radial version
      (Effects|SpawnEmitteratLocation (Variables|Default|GetEmitterToSpawnRadial) _returnvalue)))
  ;[1 1 1] Lastly we destroy the actor
  (Actor|DestroyActor))

(event EventBeginPlay
  ;[1 1 1] In case that the grenade doesn't collide with anything for 0.75 seconds we trigger the explosion
  (Utilities|FlowControl|Delay 0.75)
  ;[1 1 1] This makes sure that the explosion triggers only once
  (Utilities|FlowControl|DoOnce false
    (:Completed
      (CallFunction|Explode))))

(fn ConstructionScript)